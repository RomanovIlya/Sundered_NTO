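; Dialogue component that runs branching, data-table-driven conversations through a dialogue widget when interacted with.
; Each interaction shows the current row's line and stores the next table, row and end flag, creating the widget and enabling cursor input on first use.
; Option rows spawn choice widgets that call back to jump to another row.
; Interacting after the last line updates a hardcoded trader diary state in GI_Sundered and closes the dialogue.
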(event Custom|OptionSelected
  (params (DataTable :type Data%20Table%20Object%20Reference) (RowName :type Name))
  (bind _returnvalue (Utilities|GetDataTableRow DataTable RowName)
    (:then
      (Widget|Panel|ClearChildren (Variables|/Game/BP/Widget/WB_Dialogue.WB_Dialogue_C|GetOptionBox (Variables|Default|GetWidgetDialogue)))
      (Default|UpdateDialogue (Variables|Default|GetWidgetDialogue) (.Dialogue (Utilities|Struct|BreakDialogue_Structure _returnvalue)))
      (Variables|Default|SetRowName (.Row (Utilities|Struct|BreakDialogue_Structure _returnvalue)))
      (Variables|Default|SetDataTable (.DataTable (Utilities|Struct|BreakDialogue_Structure _returnvalue)))
      (Variables|Default|SetIs%20Dialogue%20End? (.IsDialogueEnd? (Utilities|Struct|BreakDialogue_Structure _returnvalue)))
      (Variables|Default|SetHasOption? false)
      (if (.OpenedDialogue? (Utilities|Struct|BreakDialogue_Structure _returnvalue))
        (CallFunction|UpdateOption (.DialogueOptions (Utilities|Struct|BreakDialogue_Structure _returnvalue)))))))

(event Custom|UpdateOption
  (params (Array :type Array%20of%20Optional%20Dialogue%20Structure%20Structures))
  (if (not (Variables|Default|GetHasOption?))
    (for _array_element Array
      (Variables|Default|SetHasOption? true)
      (bind _returnvalue (UserInterface|CreateWidget "/Game/BP/Widget/WB_Option.WB_Option_C" (Game|GetPlayerController 0) (.OptionName (Utilities|Struct|BreakOptionalDialogue_Structure _array_element)) self (.Database (Utilities|Struct|BreakOptionalDialogue_Structure _array_element)) (.Row (Utilities|Struct|BreakOptionalDialogue_Structure _array_element))))
      (Widget|Panel|AddChild (Variables|/Game/BP/Widget/WB_Dialogue.WB_Dialogue_C|GetOptionBox (Variables|Default|GetWidgetDialogue)) _returnvalue))))

(event EventBeginPlay)

(event EventTick
  (params (DeltaSeconds :type Float%20%28single-precision%29)))

(event EventInteract
  (params (PlayerRef :type BP%20Viking%20Object%20Reference))
  (bind _returnvalue (Game|GetPlayerController 0))
  (if (Variables|Default|GetIs%20Dialogue%20End?)
    (bind _asgi_sundered (Utilities|Casting|CastToGI_Sundered (Game|GetGameInstance)))
    (Default|UpdateDiaryState _asgi_sundered "Traider_1")
    (|EndDialogue)
    (else
      (Utilities|IsValid (Variables|Default|GetWidgetDialogue)
        (:Is%20Valid
          (bind _returnvalue_2 (Utilities|GetDataTableRow (Variables|Default|GetDataTable) (Variables|Default|GetRowName))
            (:then
              (Default|UpdateDialogue (Variables|Default|GetWidgetDialogue) (.Dialogue (Utilities|Struct|BreakDialogue_Structure _returnvalue_2)))
              (Variables|Default|SetRowName (.Row (Utilities|Struct|BreakDialogue_Structure _returnvalue_2)))
              (Variables|Default|SetDataTable (.DataTable (Utilities|Struct|BreakDialogue_Structure _returnvalue_2)))
              (Variables|Default|SetIs%20Dialogue%20End? (.IsDialogueEnd? (Utilities|Struct|BreakDialogue_Structure _returnvalue_2)))
              (if (.OpenedDialogue? (Utilities|Struct|BreakDialogue_Structure _returnvalue_2))
                (CallFunction|UpdateOption (.DialogueOptions (Utilities|Struct|BreakDialogue_Structure _returnvalue_2)))))))
        (:Is%20Not%20Valid
          (bind _returnvalue_3 (Utilities|GetDataTableRow (Variables|Default|GetDataTable) (Variables|Default|GetRowName))
            (:then
              (bind _returnvalue_4 (UserInterface|CreateWidget "/Game/BP/Widget/WB_Dialogue.WB_Dialogue_C" (Game|GetPlayerController 0) (Variables|Default|GetName) (.Dialogue (Utilities|Struct|BreakDialogue_Structure _returnvalue_3))))
              (bind _output_get (Variables|Default|SetWidgetDialogue _returnvalue_4))
              (UserInterface|Viewport|AddtoViewport _output_get 0)
              (Variables|Default|SetRowName (.Row (Utilities|Struct|BreakDialogue_Structure _returnvalue_3)))
              (Variables|Default|SetDataTable (.DataTable (Utilities|Struct|BreakDialogue_Structure _returnvalue_3)))
              (Variables|Default|SetIs%20Dialogue%20End? (.IsDialogueEnd? (Utilities|Struct|BreakDialogue_Structure _returnvalue_3)))
              (Input|SetInputModeGameandUI _returnvalue 0 "DoNotLock" true false)
              (Variables|/Script/Engine.PlayerController|SetbShowMouseCursor _returnvalue true)
              (if (.OpenedDialogue? (Utilities|Struct|BreakDialogue_Structure _returnvalue_3))
                (CallFunction|UpdateOption (.DialogueOptions (Utilities|Struct|BreakDialogue_Structure _returnvalue_3)))))))))))

(event EventEndInteract
  (Utilities|IsValid (Variables|Default|GetWidgetDialogue)
    (:Is%20Valid
      (|EndDialogue))))