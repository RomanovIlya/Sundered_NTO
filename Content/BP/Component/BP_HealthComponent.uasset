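; Health component Blueprint that handles damage and a limited number of heals for its owner.
; GetDamage subtracts damage divided by Defense from Health and returns whether Health remains above zero.
; Heal adds the given amount and decrements HealCount while that count is at least zero, then returns whether it is still non-negative.
; BeginPlay and Tick are unused, so all logic runs only when these functions are called.
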(event EventBeginPlay)

(event EventTick
  (params (DeltaSeconds :type Float%20%28single-precision%29)))

(fn GetDamage
  (params (Damage :type Float%20%28double-precision%29))
  (bind _output_get (Variables|Default|Sethealth (- (Variables|Default|Gethealth) (/ Damage (Variables|Default|Getdefense)))))
  (return (> _output_get 0.0)))

(fn Heal
  (params (health :type Float%20%28double-precision%29))
  (if (>= (Variables|Default|GetHealCount) 0)
    (Variables|Default|Sethealth (+ (Variables|Default|Gethealth) health))
    (Variables|Default|SetHealCount (- (Variables|Default|GetHealCount) 1)))
  (return (>= (Variables|Default|GetHealCount) 0)))