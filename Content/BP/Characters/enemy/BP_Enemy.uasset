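; BP_Enemy is an AI enemy that patrols, attacks BP_Viking and can be hurt and killed.
; It patrols to random X points via AI MoveTo; PawnSensing sight or noise triggers a chase and attack on arrival, with a retriggerable delay resuming patrol.
; Damage runs through BPHealthComponent, playing Hurt or Death animation overrides, then destroying the actor and calling a death event.
; CanMoving, IsAttacking and IsDead flags gate these actions.
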(event OnHearNoise(PawnSensing)
  (params (Instigator :type Pawn%20Object%20Reference) (Location :type Vector%20%28by%20ref%29 :default "0, 0, 0") (Volume :type Float%20%28single-precision%29))
  ;[0.15 0.15 0.15 0.5] Follow
  (bind _asbp_viking (Utilities|Casting|CastToBP_Viking Instigator))
  (if (not (Variables|/Game/BP/Characters/Viking/BP_Viking.BP_Viking_C|GetIsDead? _asbp_viking))
    (Utilities|FlowControl|Sequence
      (:then_0
        (AI|AIMoveTo self (Math|Vector|MakeVector 0.0 0.0 0.0) _asbp_viking 5.0 true
          (:OnSuccess
            (if (not (Variables|Default|GetIsAttacking))
              (CallFunction|Attack)))))
      (:then_1
        (Utilities|FlowControl|RetriggerableDelay 1.0)
        (CallFunction|Moving)))))

(event OnSeePawn(PawnSensing)
  (params (Pawn :type Pawn%20Object%20Reference))
  ;[0.15 0.15 0.15 0.5] Follow
  (bind _asbp_viking (Utilities|Casting|CastToBP_Viking (stale OnHearNoise(PawnSensing) Instigator)))
  (if (not (Variables|/Game/BP/Characters/Viking/BP_Viking.BP_Viking_C|GetIsDead? _asbp_viking))
    (Utilities|FlowControl|Sequence
      (:then_0
        (AI|AIMoveTo self (Math|Vector|MakeVector 0.0 0.0 0.0) _asbp_viking 5.0 true
          (:OnSuccess
            (if (not (Variables|Default|GetIsAttacking))
              (CallFunction|Attack)))))
      (:then_1
        (Utilities|FlowControl|RetriggerableDelay 1.0)
        (CallFunction|Moving)))))

(event Custom|Moving
  (bind _returnvalue (Transformation|GetActorLocation))
  (bind (_x _y _z) (Math|Vector|BreakVector _returnvalue))
  ;[0.15 0.15 0.15 0.5] Patrol Location
  (if (Variables|Default|GetCanMoving?)
    (AI|AIMoveTo self (Math|Vector|MakeVector (.x (.RandomLocation (AI|Navigation|GetRandomReachablePointinRadius _returnvalue 5e+02 0 0))) _y _z) 0 5.0 false
      (:OnSuccess
        (Utilities|FlowControl|Delay 2.0)
        (CallFunction|Moving)))))

(event Custom|Attack
  (if (Variables|Default|GetCanMoving?)
    (Variables|Default|SetCanMoving? false)
    (Variables|Default|SetIsAttacking true)
    (|PlayAnimationOverridewithCallbacks (Variables|/Script/PaperZD.PaperZDAnimationComponent|GetAnimInstance (Variables|Default|GetAnimationComponent)) (Variables|Default|GetAttack) "DefaultSlot" 1.0 0.0
      (:OnCompleted
        _)
      (:OnCancelled
        _))
    (Variables|Default|SetIsAttacking false)
    (Variables|Default|SetCanMoving? true)))

(event EventBeginPlay
  (Default|CallOnSpawned)
  (CallFunction|Moving))

(event Collision|EventActorBeginOverlap
  (params (OtherActor :type Actor%20Object%20Reference)))

(event EventTick
  (params (DeltaSeconds :type Float%20%28single-precision%29)))

(event Game|Damage|EventAnyDamage
  (params (Damage :type Float%20%28single-precision%29) (DamageType :type Damage%20Type%20Object%20Reference) (InstigatedBy :type Controller%20Object%20Reference) (DamageCauser :type Actor%20Object%20Reference))
  ;[0.15 0.15 0.15 0.5] OnAnyDamge
  (if (and (> (Variables|/Game/BP/Component/BP_HealthComponent.BP_HealthComponent_C|Gethealth (Variables|Default|GetBP_HealthComponent)) 0.0) (not (Variables|Default|GetIsDead?)))
    (Variables|Default|SetCanMoving? false)
    (bind _islive_ (Default|GetDamage (Variables|Default|GetBP_HealthComponent) Damage))
    (if _islive_
      (|PlayAnimationOverridewithCallbacks (Variables|/Script/PaperZD.PaperZDAnimationComponent|GetAnimInstance (Variables|Default|GetAnimationComponent)) (Variables|Default|GetHurt) "DefaultSlot" 1.0 0.0
        (:OnCompleted
          (Variables|Default|SetCanMoving? true)))
      (else
        (Variables|Default|SetIsDead? true)
        (|PlayAnimationOverridewithCallbacks (Variables|/Script/PaperZD.PaperZDAnimationComponent|GetAnimInstance (Variables|Default|GetAnimationComponent)) (Variables|Default|GetDeath) "DefaultSlot" 1.0 0.0
          (:OnCompleted
            _)
          (:OnCancelled
            _))
        (Actor|DestroyActor)
        (Default|CallDeathEvent)))
    (else
      (Variables|Default|SetIsDead? true)
      (|PlayAnimationOverridewithCallbacks (Variables|/Script/PaperZD.PaperZDAnimationComponent|GetAnimInstance (Variables|Default|GetAnimationComponent)) (Variables|Default|GetDeath) "DefaultSlot" 1.0 0.0
        (:OnCompleted
          _)
        (:OnCancelled
          _))
      (Actor|DestroyActor)
      (Default|CallDeathEvent))))

(event EventPossessed
  (params (NewController :type Controller%20Object%20Reference))
  (Default|CallOnSpawned)
  (CallFunction|Moving))

(fn ConstructionScript)