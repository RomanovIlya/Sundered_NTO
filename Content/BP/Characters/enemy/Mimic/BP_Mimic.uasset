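; BP_Mimic is an enemy character that takes damage from BP_Viking and summons orc reinforcements.
; Damage from the Viking goes to BPHealthComponent, and a successful result jumps the PaperZD animation to its Hurt node.
; Tick prints health and, when it exactly equals three quarters of maximum, increments Stage and spawns two BP_Orc2 at the mesh's transform.
; Clearing CanDamage makes that summon one-time, as nothing here resets it.
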(event EventBeginPlay)

(event Game|Damage|EventAnyDamage
  (params (Damage :type Float%20%28single-precision%29) (DamageType :type Damage%20Type%20Object%20Reference) (InstigatedBy :type Controller%20Object%20Reference) (DamageCauser :type Actor%20Object%20Reference))
  (Utilities|Casting|CastToBP_Viking DamageCauser)
  (bind _islive_ (Default|GetDamage (Variables|Default|GetBP_HealthComponent) Damage))
  (if _islive_
    (Class|PaperZDAnimInstance|JumptoNode (Variables|/Script/PaperZD.PaperZDAnimationComponent|GetAnimInstance (Variables|Default|GetPaperZDAnimation)) "Hurt" "None")))

(event EventTick
  (params (DeltaSeconds :type Float%20%28single-precision%29))
  (bind _bp_healthcomponent (Variables|Default|GetBP_HealthComponent))
  (bind _max_health (Variables|/Game/BP/Component/BP_HealthComponent.BP_HealthComponent_C|Getmax_health _bp_healthcomponent))
  (bind _health (Variables|/Game/BP/Component/BP_HealthComponent.BP_HealthComponent_C|Gethealth _bp_healthcomponent))
  (Development|PrintString (Utilities|String|ToString(Float) _health))
  (if (and (== (- _max_health (/ _max_health 4.0)) _health) (Variables|Default|GetCanDamage?))
    (Variables|Default|Setstage (+ (Variables|Default|Getstage) 1))
    (Variables|Default|SetCanDamage? false)
    (Utilities|FlowControl|Sequence
      (:then_0
        (Game|SpawnActorfromClass "/Game/BP/Characters/enemy/Orc_2/BP_Orc2.BP_Orc2_C" (Transformation|GetWorldTransform (Variables|Default|GetStaticMesh)) "Undefined" "MultiplyWithRoot" 0 0))
      (:then_1
        (Game|SpawnActorfromClass "/Game/BP/Characters/enemy/Orc_2/BP_Orc2.BP_Orc2_C" (Transformation|GetWorldTransform (Variables|Default|GetStaticMesh)) "Undefined" "MultiplyWithRoot" 0 0)))))

(fn ConstructionScript)