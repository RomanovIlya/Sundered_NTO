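; Mimic boss enemy that starts battle music, flags the player as in battle and repeats a PaperZD attack animation on a delayed loop until dead.
; Tick checks health against quarter-step thresholds, each making it invulnerable and spawning two orcs whose death events restore damage once both die.
; Death attaches a dialogue component and hands it to the player; when dialogue ends, the screen fades and the Cut2 level loads.
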(event Custom|Attack
  (if (not (Variables|Default|GetDead?))
    (Variables|Default|SetIsAttacking? true)
    (|PlayAnimationOverridewithCallbacks (Variables|/Script/PaperZD.PaperZDAnimationComponent|GetAnimInstance (Variables|Default|GetAnimationComponent)) "/Game/BP/Characters/enemy/Mimic/AnimSequences/attack.attack" "DefaultSlot" 1.0 0.0
      (:OnCompleted
        (Variables|Default|SetIsAttacking? false)
        (Utilities|FlowControl|Delay 6.0)
        (CallFunction|Attack)))))

(event Custom|Death
  (Variables|Default|SetDead? true)
  (Class|PaperZDAnimInstance|JumptoNode (Variables|/Script/PaperZD.PaperZDAnimationComponent|GetAnimInstance (Variables|Default|GetAnimationComponent)) "Death" "None")
  (bind _returnvalue (Game|AddComponentbyClass "/Game/BP/Component/BP_DialogueComponent.BP_DialogueComponent_C"))
  (Variables|Default|SetDialogue _returnvalue)
  (Variables|/Game/BP/Component/BP_DialogueComponent.BP_DialogueComponent_C|SetName _returnvalue "Мимик")
  (Variables|/Game/BP/Component/BP_DialogueComponent.BP_DialogueComponent_C|SetRowName _returnvalue "1")
  (Variables|/Game/BP/Component/BP_DialogueComponent.BP_DialogueComponent_C|SetDataTable _returnvalue "/Game/BP/Dialogue/Mimic2.Mimic2")
  (bind _asbp_viking (Utilities|Casting|CastToBP_Viking (Game|Player|GetPlayerPawn 0)))
  (Variables|/Game/BP/Characters/Viking/BP_Viking.BP_Viking_C|SetD_Actor _asbp_viking _returnvalue)
  (Rendering|SetVisibility (Variables|Default|GetWidget) true false))

(event EventBeginPlay
  (Utilities|FlowControl|Sequence
    (:then_0
      (CallFunction|Attack))
    (:then_1
      (Audio|PlaySound2D "/Game/Assets/Music/BattleMusic.BattleMusic" 1.0 1.0 0.0 0 0))
    (:then_2
      (bind _asbp_viking (Utilities|Casting|CastToBP_Viking (Game|Player|GetPlayerPawn 0)))
      (Variables|/Game/BP/Characters/Viking/BP_Viking.BP_Viking_C|SetIsInBattle? _asbp_viking true))))

(event Collision|EventActorBeginOverlap
  (params (OtherActor :type Actor%20Object%20Reference)))

(event Game|Damage|EventAnyDamage
  (params (Damage :type Float%20%28single-precision%29) (DamageType :type Damage%20Type%20Object%20Reference) (InstigatedBy :type Controller%20Object%20Reference) (DamageCauser :type Actor%20Object%20Reference))
  (if (Variables|Default|GetCanDamage?)
    (bind _islive_ (Default|GetDamage (Variables|Default|GetBP_HealthComponent) Damage))
    (if _islive_
      (if (not (Variables|Default|GetIsAttacking?))
        (Class|PaperZDAnimInstance|JumptoNode (Variables|/Script/PaperZD.PaperZDAnimationComponent|GetAnimInstance (Variables|Default|GetAnimationComponent)) "Hurt" "None"))
      (else
        (CallFunction|Death)))))

(event EventTick
  (params (DeltaSeconds :type Float%20%28single-precision%29))
  (bind _dialogue (Variables|Default|GetDialogue))
  (Utilities|FlowControl|Sequence
    (:then_0
      (|SpawActors))
    (:then_1
      (Utilities|IsValid _dialogue
        (:Is%20Valid
          (if (Variables|/Game/BP/Component/BP_DialogueComponent.BP_DialogueComponent_C|GetIs%20Dialogue%20End? _dialogue)
            (Utilities|FlowControl|Delay 1e+01)
            (bind _returnvalue (UserInterface|CreateWidget "/Game/BP/Widget/WB_FadeInOut.WB_FadeInOut_C" (Game|GetPlayerController 0) true false))
            (UserInterface|Viewport|AddtoViewport _returnvalue 0)
            (Utilities|FlowControl|Delay 0.5)
            (Game|OpenLevel(byObjectReference) "/Game/Maps/Cut2.Cut2")))))))

(fn ConstructionScript)

(event Custom|DeathMim
  (Variables|Default|SetEnemyCount (- (Variables|Default|GetEnemyCount) 1))
  (if (<= (Variables|Default|GetEnemyCount) 0)
    (Class|PaperZDAnimInstance|JumptoNode (Variables|/Script/PaperZD.PaperZDAnimationComponent|GetAnimInstance (Variables|Default|GetAnimationComponent)) "Angry" "None")
    (Variables|Default|SetCanDamage? true)))