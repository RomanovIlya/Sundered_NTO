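; BP_EnemySpawner is a trigger-driven spawner that populates an area and seals it when BP_Viking overlaps its Box.
; Each overlap spawns every class in Actors at random reachable nav points within Radius, keeping the spawner's Y so spawns share one plane.
; It then sets Box1 and Box2 to block all channels; nothing here reopens them or prevents retriggering.
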(event OnComponentBeginOverlap(Box)
  (params (OverlappedComponent :type Primitive%20Component%20Object%20Reference) (OtherActor :type Actor%20Object%20Reference) (OtherComp :type Primitive%20Component%20Object%20Reference) (OtherBodyIndex :type Integer) (bFromSweep :type Boolean) (SweepResult :type Hit%20Result%20Structure%20%28by%20ref%29))
  (bind _returnvalue (Transformation|GetActorLocation))
  (Utilities|Casting|CastToBP_Viking OtherActor)
  (Utilities|FlowControl|Sequence
    (:then_0
      (for _array_element (Variables|Default|GetActors)
        (bind _randomlocation (AI|Navigation|GetRandomReachablePointinRadius _returnvalue (Variables|Default|GetRadius) 0 0))
        (Game|SpawnActorfromClass _array_element (Math|Transform|MakeTransform (Math|Vector|MakeVector (.x _randomlocation) (.Y (Math|Vector|BreakVector _returnvalue)) (.z _randomlocation)) "0, 0, 0" "1.000000,1.000000,1.000000") "AdjustIfPossibleButDontSpawnIfColliding" "MultiplyWithRoot" 0 0)))
    (:then_1
      (Collision|SetCollisionResponsetoAllChannels (Variables|Default|GetBox1) "ECR_Block")
      (Collision|SetCollisionResponsetoAllChannels (Variables|Default|GetBox2) "ECR_Block"))))

(event EventBeginPlay)

(event Collision|EventActorBeginOverlap
  (params (OtherActor :type Actor%20Object%20Reference)))

(event EventTick
  (params (DeltaSeconds :type Float%20%28single-precision%29)))

(fn ConstructionScript)