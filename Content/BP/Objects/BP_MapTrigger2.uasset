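; BP_MapTrigger2 is a level transition trigger that sends the player to the level referenced by BossLoc.
; When BP_Viking enters the Box, it shows a WB_FadeInOut fade widget and waits briefly.
; It then clears HaveSave on GI_Sundered, calls OnCloseLevel, requests a non-blocking stream load of BossLoc and immediately opens that level.
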(event OnComponentBeginOverlap(Box)
  (params (OverlappedComponent :type Primitive%20Component%20Object%20Reference) (OtherActor :type Actor%20Object%20Reference) (OtherComp :type Primitive%20Component%20Object%20Reference) (OtherBodyIndex :type Integer) (bFromSweep :type Boolean) (SweepResult :type Hit%20Result%20Structure%20%28by%20ref%29))
  (Utilities|Casting|CastToBP_Viking OtherActor)
  (bind _returnvalue (UserInterface|CreateWidget "/Game/BP/Widget/WB_FadeInOut.WB_FadeInOut_C" (Game|GetPlayerController 0) true false))
  (UserInterface|Viewport|AddtoViewport _returnvalue 0)
  (Utilities|FlowControl|Delay 0.5)
  (bind _asgi_sundered (Utilities|Casting|CastToGI_Sundered (Game|GetGameInstance)))
  (Variables|/Game/BP/GameInstance/GI_Sundered.GI_Sundered_C|SetHaveSave? _asgi_sundered false)
  (Default|OnCloseLevel _asgi_sundered)
  (Class|GameplayStatics|LoadStreamLevelbySoftObjectPtr "/Game/Maps/BossLoc.BossLoc" false false)
  (Game|OpenLevel(byObjectReference) "/Game/Maps/BossLoc.BossLoc"))

(event EventBeginPlay)

(event Collision|EventActorBeginOverlap
  (params (OtherActor :type Actor%20Object%20Reference)))

(event EventTick
  (params (DeltaSeconds :type Float%20%28single-precision%29)))

(fn ConstructionScript)