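; BP_Boat is an interactable boat that teleports the player to the level's first found TargetPoint, once the first found BP_NPC's dialogue row is "12".
; Its sphere overlap shows an interaction prompt to BP_Viking under that dialogue condition.
; Interact locks movement and input behind a WB_FadeInOut widget, then teleports after a short delay.
; Tick polls the widget for completion, then removes it and restores control.
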(event OnComponentBeginOverlap(Sphere)
  (params (OverlappedComponent :type Primitive%20Component%20Object%20Reference) (OtherActor :type Actor%20Object%20Reference) (OtherComp :type Primitive%20Component%20Object%20Reference) (OtherBodyIndex :type Integer) (bFromSweep :type Boolean) (SweepResult :type Hit%20Result%20Structure%20%28by%20ref%29))
  (bind _outactors (Actor|GetAllActorsOfClass "/Game/BP/Characters/NPC/BP_NPC.BP_NPC_C"))
  (if (== (Variables|/Game/BP/Component/BP_DialogueComponent.BP_DialogueComponent_C|GetRowName (Variables|/Game/BP/Characters/NPC/BP_NPC.BP_NPC_C|GetBP_DialogueComponent (Utilities|Array|Get(acopy) _outactors))) "12")
    (Utilities|Casting|CastToBP_Viking OtherActor)
    (Rendering|SetVisibility (Variables|Default|GetInteraction) true false)))

(event OnComponentEndOverlap(Sphere)
  (params (OverlappedComponent :type Primitive%20Component%20Object%20Reference) (OtherActor :type Actor%20Object%20Reference) (OtherComp :type Primitive%20Component%20Object%20Reference) (OtherBodyIndex :type Integer))
  (Utilities|Casting|CastToBP_Viking OtherActor)
  (Rendering|SetVisibility (Variables|Default|GetInteraction) false false))

(event EventBeginPlay)

(event Collision|EventActorBeginOverlap
  (params (OtherActor :type Actor%20Object%20Reference)))

(event EventTick
  (params (DeltaSeconds :type Float%20%28single-precision%29))
  (Utilities|IsValid (Variables|Default|GetWidget)
    (:Is%20Valid
      (if (Variables|/Game/BP/Widget/WB_FadeInOut.WB_FadeInOut_C|GetComplete (Variables|Default|GetWidget))
        (Utilities|FlowControl|Delay 0.4)
        (Widget|RemovefromParent (Variables|Default|GetWidget))
        (Variables|Default|SetWidget 0)
        (Variables|/Game/BP/Characters/Viking/BP_Viking.BP_Viking_C|SetIsMovementLock? (Variables|Default|GetPlayer%20Ref) false)
        (Input|SetInputModeGameOnly (Game|GetPlayerController 0) false)))))

(event EventInteract
  (params (PlayerRef :type BP%20Viking%20Object%20Reference))
  (bind _returnvalue (Game|GetPlayerController 0))
  (Variables|Default|SetPlayer%20Ref PlayerRef)
  (bind _outactors (Actor|GetAllActorsOfClass "/Game/BP/Characters/NPC/BP_NPC.BP_NPC_C"))
  (if (== (Variables|/Game/BP/Component/BP_DialogueComponent.BP_DialogueComponent_C|GetRowName (Variables|/Game/BP/Characters/NPC/BP_NPC.BP_NPC_C|GetBP_DialogueComponent (Utilities|Array|Get(acopy) _outactors))) "12")
    (bind _returnvalue_2 (UserInterface|CreateWidget "/Game/BP/Widget/WB_FadeInOut.WB_FadeInOut_C" _returnvalue true))
    (Variables|Default|SetWidget _returnvalue_2)
    (UserInterface|Viewport|AddtoViewport _returnvalue_2 0)
    (Input|SetInputModeUIOnly _returnvalue 0 "DoNotLock" false)
    (Variables|/Game/BP/Characters/Viking/BP_Viking.BP_Viking_C|SetIsMovementLock? (Variables|Default|GetPlayer%20Ref) true)
    (Variables|/Script/Engine.MovementComponent|SetVelocity (Variables|/Script/Engine.Character|GetCharacterMovement (Variables|Default|GetPlayer%20Ref)) "0, 0, 0")
    (bind _outactors_2 (Actor|GetAllActorsOfClass "/Script/Engine.TargetPoint"))
    (Utilities|FlowControl|Delay 0.7)
    (Transformation|SetActorLocation (Variables|Default|GetPlayer%20Ref) (Transformation|GetActorLocation (Utilities|Array|Get(acopy) _outactors_2)) false true)))

(fn ConstructionScript)