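; Bandage pickup actor that the player collects by interacting with it.
; On Interact it clears the player's interacting flag and stores its own class, not the instance, in the player's PickableObjects.
; It then updates the "Bandage" diary state through the GI_Sundered game instance and destroys itself; if that cast fails, the actor stays in the world.
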(event EventBeginPlay
  (|CallParentFunction) ; This node is disabled and will not be called.\nDrag off pins to build functionality.
)

(event Collision|EventActorBeginOverlap
  (params (OtherActor :type Actor%20Object%20Reference))
  (|CallParentFunction OtherActor) ; This node is disabled and will not be called.\nDrag off pins to build functionality.
)

(event EventTick
  (params (DeltaSeconds :type Float%20%28single-precision%29))
  (|CallParentFunction DeltaSeconds) ; This node is disabled and will not be called.\nDrag off pins to build functionality.
)

(event EventInteract
  (params (PlayerRef :type BP%20Viking%20Object%20Reference))
  (Variables|/Game/BP/Characters/Viking/BP_Viking.BP_Viking_C|SetIsIntercting? PlayerRef false)
  (Utilities|Array|Add (Variables|/Game/BP/Characters/Viking/BP_Viking.BP_Viking_C|GetPickableObjects PlayerRef) (Utilities|GetClass self))
  (bind _asgi_sundered (Utilities|Casting|CastToGI_Sundered (Game|GetGameInstance)))
  (Default|UpdateDiaryState _asgi_sundered "Bandage")
  (Actor|DestroyActor))

(fn ConstructionScript
  (|CallParentFunction))